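; Character Blueprint that uses the Gameplay Ability System for health and shield, shown on a locally controlled HUD widget.
; BeginPlay creates the HUD, and attribute-change events push current and max values to it.
; The jump input applies a SetByCaller damage effect to the character itself instead of jumping, apparently as a test trigger.
; Movement is disabled when health reaches zero.
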(event `self.ReceiveBeginPlay`
  (if (`self.IsLocallyControlled`)
    (bind _returnvalue (`|CreateWidget` "/Game/UI/WBP_HUD.WBP_HUD_C"))
    (bind _output_get (set `self.WBP_HUD` _returnvalue))
    (`UserWidget.AddToViewport` _output_get 0)
    (`self.UpdateHealth`)
    (`self.UpdateShield`)))

(event `EnhancedInput|/Game/Characters/Input/IA_Jump`
  (params (ActionValue :type Boolean) (ElapsedSeconds :type "Float (double-precision)") (TriggeredSeconds :type "Float (double-precision)") (InputAction :type "InputAction Object Reference" :default "/Game/Characters/Input/IA_Jump.IA_Jump"))
  (bind _abilitysystemcomponent (`self.AbilitySystemComponent`))
  (:`Started`
    (bind _returnvalue (`AbilitySystemBlueprintLibrary.AssignTagSetByCallerMagnitude` (`AbilitySystemComponent.MakeOutgoingSpec` :`self` _abilitysystemcomponent :`GameplayEffectClass` "/Game/GAS/Effects/GE_Damage.GE_Damage_C") (struct :`TagName` "Damage.SetByCaller") 20.0))
    (`AbilitySystemComponent.BP_ApplyGameplayEffectSpecToSelf` _abilitysystemcomponent _returnvalue)))

(event `self.OnHealthChanged`
  (params (OldValue :type "Float (single-precision)") (NewValue :type "Float (single-precision)"))
  (`self.UpdateHealth`)
  (if (<= NewValue 0.0)
    (`CharacterMovementComponent.DisableMovement` (`self.CharacterMovement`))))

(event `self.OnShieldChanged`
  (params (OldValue :type "Float (single-precision)") (NewValue :type "Float (single-precision)"))
  (`self.UpdateShield`))

(fn `UpdateHealth`
  (bind _abilitysystemcomponent (`self.AbilitySystemComponent`))
  (if (`self.IsLocallyControlled`)
    (`/Game/UI/WBP_HUD.UpdateHealth` (`self.WBP_HUD`) (`.ReturnValue` (`AbilitySystemComponent.GetGameplayAttributeValue` _abilitysystemcomponent (struct :`AttributeName` "Health" :`Attribute` "/Script/GG.GGHealthSet:Health" :`AttributeOwner` "/Script/CoreUObject.Class'/Script/GG.GGHealthSet'"))) (`.ReturnValue` (`AbilitySystemComponent.GetGameplayAttributeValue` _abilitysystemcomponent (struct :`AttributeName` "MaxHealth" :`Attribute` "/Script/GG.GGHealthSet:MaxHealth" :`AttributeOwner` "/Script/CoreUObject.Class'/Script/GG.GGHealthSet'"))))))

(fn `UpdateShield`
  (locals (NewLocalVar :type "/Game/UI/WBP_HUD Object Reference"))
  (bind _abilitysystemcomponent (`self.AbilitySystemComponent`))
  (bind _wbp_hud (`self.WBP_HUD`))
  (if (`KismetSystemLibrary.IsValid` _wbp_hud)
    (if (`self.IsLocallyControlled`)
      (`/Game/UI/WBP_HUD.UpdateShield` _wbp_hud (`.ReturnValue` (`AbilitySystemComponent.GetGameplayAttributeValue` _abilitysystemcomponent (struct :`AttributeName` "Shield" :`Attribute` "/Script/GG.GGHealthSet:Shield" :`AttributeOwner` "/Script/CoreUObject.Class'/Script/GG.GGHealthSet'"))) (`.ReturnValue` (`AbilitySystemComponent.GetGameplayAttributeValue` _abilitysystemcomponent (struct :`AttributeName` "MaxShield" :`Attribute` "/Script/GG.GGHealthSet:MaxShield" :`AttributeOwner` "/Script/CoreUObject.Class'/Script/GG.GGHealthSet'")))))))

(fn `UserConstructionScript`)