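; GA_FireAbility is a Gameplay Ability that fires a hitscan shot from the character's camera to deal damage.
; After committing, it line-traces on the Camera channel from the camera toward its scaled forward vector, which is not offset by the camera location.
; A hit actor with an ability system component receives GE_Damage with a fixed SetByCaller magnitude.
; The ability then ends immediately, as it does when commit fails.
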(event `self.K2_ActivateAbility`
  (bind _returnvalue (`self.GetAbilitySystemComponentFromActorInfo`))
  (bind _cameracomp (`GGPlayerCharacter.CameraComp` (`self.Character`)))
  (bind _asbp_character (cast `/Game/Characters/BP_Character` (`self.GetAvatarActorFromActorInfo`)))
  (set `self.Character` _asbp_character)
  (bind _returnvalue_2 (`self.K2_CommitAbility`))
  (if _returnvalue_2
    (`|ExecutionSequence`
      (:`then_0`
        (bind _outhit (`KismetSystemLibrary.LineTraceSingle` (`SceneComponent.K2_GetComponentLocation` _cameracomp) (* (`KismetMathLibrary.GetForwardVector` (`SceneComponent.K2_GetComponentRotation` _cameracomp)) 5000.0) "TraceTypeQuery2"))
        (bind _returnvalue_3 (`AbilitySystemBlueprintLibrary.GetAbilitySystemComponent` (`.HitActor` (`GameplayStatics.BreakHitResult` _outhit))))
        (`/Engine/EditorBlueprintResources/StandardMacros.IsValid` _returnvalue_3
          (:`Is Valid`
            (bind _returnvalue_4 (`AbilitySystemBlueprintLibrary.AssignTagSetByCallerMagnitude` (`AbilitySystemComponent.MakeOutgoingSpec` :`self` _returnvalue :`GameplayEffectClass` "/Game/GAS/Effects/GE_Damage.GE_Damage_C") (struct :`TagName` "Damage.SetByCaller") 10.0))
            (`AbilitySystemComponent.BP_ApplyGameplayEffectSpecToTarget` _returnvalue _returnvalue_4 _returnvalue_3))))
      (:`then_1`
        (`self.K2_EndAbility` :!label _label)))
    (else
      (goto _label))))